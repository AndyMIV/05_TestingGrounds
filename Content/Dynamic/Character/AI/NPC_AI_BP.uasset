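; AI controller for guard NPCs that runs the GuardBehaviour behavior tree on the PatrolData blackboard from BeginPlay.
; AI Perception updates feed UpdateBlackboardEnemyKey, which ignores actors tagged "Enemy", stores other sensed actors as the enemy key and clears it when sensing fails.
; Earlier patrol, targeting and shooting logic remains as unconnected nodes, with shooting noted as moved to a ShootAtEnemy service.
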(event OnTargetPerceptionUpdated(AIPerception)
  (params (Actor :type Actor%20Object%20Reference) (Stimulus :type AI%20Stimulus%20Structure))
  (CallFunction|UpdateBlackboardEnemyKey Stimulus Actor))

(event EventBeginPlay
  ;[1 1 1] Find Patrol Route
  (bind _blackboardcomponent (Class|AIController|UseBlackboard "/Game/Dynamic/Character/AI/PatrolData.PatrolData"))
  (AI|RunBehaviorTree "/Game/Dynamic/Character/AI/GuardBehaviour.GuardBehaviour")
  (Variables|Default|SetBlackboardComp _blackboardcomponent))

(fn ConstructionScript)

(fn FindPatrolRoute
  (params (BlackBoard :type Blackboard%20Component%20Object%20Reference)))

(fn UpdateBlackboardEnemyKey
  (params (AIStimulus :type AI%20Stimulus%20Structure%20%28by%20ref%29) (ActorRef1 :type Actor%20Object%20Reference))
  (bind _blackboardcomp (Variables|Default|GetBlackboardComp))
  (bind _enemykey (Variables|Default|GetEnemyKey))
  (if (not (Actor|ActorHasTag ActorRef1 "Enemy"))
    (if (.bSuccessfullySensed (Utilities|Struct|BreakAIStimulus AIStimulus))
      (AI|Components|Blackboard|SetValueasObject _blackboardcomp _enemykey ActorRef1)
      (Development|PrintString "Set Value As Object Sucessful")
      (else
        (AI|Components|Blackboard|ClearValue _blackboardcomp _enemykey)
        (Development|PrintString "Lost Target")))))